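; BP_P38 is a P-38 plane actor that flies forward continuously while its two propellers spin.
; Each tick it moves along its local X axis at MoveSpeed, scaled by delta time.
; It then calls a shared RotatePropeller function for the Left and Right propellers, adding frame-rate-independent roll at PropellerRotateSpeed.
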(event EventTick
  (params (DeltaSeconds :type Float%20%28single-precision%29))
  (Utilities|FlowControl|Sequence
    (:then_0
      (Transformation|AddActorLocalOffset (Math|Vector|MakeVector (* DeltaSeconds (Variables|Speed|GetMoveSpeed)) 0.0 0.0) false false))
    (:then_1
      (CallFunction|RotatePropeller (Variables|Default|GetLeft)))
    (:then_2
      (CallFunction|RotatePropeller (Variables|Default|GetRight)))))

(fn ConstructionScript)

(fn RotatePropeller
  (params (where :type Static%20Mesh%20Component%20Object%20Reference))
  (Transformation|AddRelativeRotation where (Math|Rotator|MakeRotator (* (Utilities|Time|GetWorldDeltaSeconds) (Variables|Speed|GetPropellerRotateSpeed)) 0.0 0.0) false false))